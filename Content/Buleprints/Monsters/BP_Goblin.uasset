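; BP_Goblin is a goblin monster Blueprint with AI perception, apparently an unfinished enemy.
; When a perception update is anything other than a successfully sensed Player-tagged actor, it starts a line-of-sight timer stored in EnemyTimer, with no event shown bound.
; AttackAni stores attack, idle and move animations passed to it.
; Sensing the player triggers nothing here, and UpdateWalkSpeed and the other events are empty.
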(event `self.AIPerception.OnTargetPerceptionUpdated`
  (params (Actor :type "Actor Object Reference") (Stimulus :type "AIStimulus Structure"))
  (if (not (and (`self.ActorHasTag` Actor "Player") (`.bSuccessfullySensed` (break `AIStimulus` Stimulus))))
    (bind _returnvalue (`KismetSystemLibrary.K2_SetTimerDelegate` :`Time` (`self.Line of Sight Time`)))
    (set `self.Enemy Timer` _returnvalue)))

(event `self.AIPerception.OnTargetPerceptionForgotten`
  (params (Actor :type "Actor Object Reference")))

(fn `AttackAni`
  (params (AttackAni :type Boolean) (IdleAni :type Boolean) (MoveAni :type Boolean))
  (set `self.bAttack` AttackAni)
  (set `self.bIdle` IdleAni)
  (set `self.bMove` MoveAni))

(fn `UpdateWalkSpeed`)

(fn `UserConstructionScript`)